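; BP_KnightPrisoner is a knight prisoner NPC that plays a looping idle animation on its skeletal mesh from BeginPlay.
; Interact prints a debug greeting, awards EarnedXP to the instigator's GD_PlayerState, then switches the mesh to a looping cheer animation through CharacterCheer.
; CanInteract always returns false, and Interact itself has no guard against repeated XP awards.
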(event Custom|CharacterCheer
  (Components|Animation|PlayAnimation (Variables|Default|GetSkeletalMesh) (Variables|Default|GetMontageCheer) true))

(event EventBeginPlay
  (Components|Animation|PlayAnimation (Variables|Default|GetSkeletalMesh) (Variables|Default|GetMontageIdle) true))

(event EventInteract
  (params (CharacterInstigator :type GD%20Character%20Object%20Reference))
  (Development|PrintString "Hello")
  (bind _asgd_player_state (Utilities|Casting|CastToGD_PlayerState (Variables|/Script/Engine.Pawn|GetPlayerState CharacterInstigator)))
  (Class|GDPlayerState|AddXp _asgd_player_state (Variables|Default|GetEarnedXP))
  (CallFunction|CharacterCheer))

(fn ConstructionScript)

(fn CanInteract
  (params (CharacterInstigator :type GD%20Character%20Object%20Reference))
  (return false))